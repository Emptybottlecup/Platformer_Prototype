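; BP_Ball is a platformer actor that rotates to aim at the mouse cursor.
; BeginPlay shows the cursor, then every Tick traces under it against one object type and computes a look-at rotation from the actor to the hit location.
; The look-at pitch drives the actor's roll, mirrored when look-at yaw exceeds a threshold to cover both sides, while the actor's pitch and yaw stay unchanged.
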(event EventBeginPlay
  (Variables|/Script/Engine.PlayerController|SetbShowMouseCursor (Game|GetPlayerController 0) true))

(event Collision|EventActorBeginOverlap
  (params (OtherActor :type Actor%20Object%20Reference)))

(event EventTick
  (params (DeltaSeconds :type Float%20%28single-precision%29))
  (bind _returnvalue (Transformation|GetActorLocation))
  (bind _returnvalue_2 (Transformation|GetActorRotation))
  (bind _returnvalue_3 (Game|GetPlayerController 0))
  (bind _array (Utilities|Array|MakeArray "ObjectTypeQuery7"))
  (bind _hitresult (Class|PlayerController|GetHitResultUnderCursorforObjects _returnvalue_3 _array true))
  (bind _returnvalue_4 (Math|Rotator|FindLookatRotation _returnvalue (.location _hitresult)))
  (if (> (.yaw _returnvalue_4) 5e+01)
    (Transformation|SetActorRotation (Math|Rotator|MakeRotator (+ (- 9e+01 (.pitch _returnvalue_4)) 9e+01) (.pitch _returnvalue_2) (.yaw _returnvalue_2)))
    (else
      (Transformation|SetActorRotation (Math|Rotator|MakeRotator (.pitch _returnvalue_4) (.pitch _returnvalue_2) (.yaw _returnvalue_2))))))

(fn ConstructionScript)